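; Weapon actor that fires a Bala projectile from PuntoDeSpawnProyectil on the Disparar input, with a debug print.
; EquiparArma attaches it to the player mesh's PistolaSkt socket and flags Policía as armed; SoltarArma detaches it and clears the flag.
; Pickup overlap events are empty, and the equip, drop, input toggle and timer-based automatic fire calls are left disconnected, with Fuego empty.
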(event `self.ReceiveActorBeginOverlap`
  (params (OtherActor :type "Actor Object Reference")))

(event `self.Colisión.OnComponentBeginOverlap`
  (params (OverlappedComponent :type "PrimitiveComponent Object Reference") (OtherActor :type "Actor Object Reference") (OtherComp :type "PrimitiveComponent Object Reference") (OtherBodyIndex :type Integer) (bFromSweep :type Boolean) (SweepResult :type "HitResult Structure (by ref)"))
  ;[1 1 1] Tomar Arma
)

(event `Key|LeftMouseButton`
  (params (Key :type "Key Structure")))

(event `self.Colisión.OnComponentEndOverlap`
  (params (OverlappedComponent :type "PrimitiveComponent Object Reference") (OtherActor :type "Actor Object Reference") (OtherComp :type "PrimitiveComponent Object Reference") (OtherBodyIndex :type Integer))
  ;[1 1 1] Tomar Arma
)

(event `InputAction|Disparar`
  (params (Key :type "Key Structure"))
  (:`Pressed`
    (`KismetSystemLibrary.PrintString` "Disparo")
    (`|SpawnActorFromClass` "/Game/Armas/Pistola/Proyectil/Bala.Bala_C" (`SceneComponent.K2_GetComponentToWorld` (`self.PuntoDeSpawnProyectil`)) "Undefined" "OverrideRootScale" null null)))

(event `InputAction|TomarArma`
  (params (Key :type "Key Structure"))
  ;[1 1 1] Tomar Arma
)

(event `Fuego`)

(event `InputAction|SoltarArma`
  (params (Key :type "Key Structure"))
  ;[1 1 1] Tomar Arma
)

(fn `EquiparArma`
  (bind _returnvalue (`GameplayStatics.GetPlayerCharacter` 0))
  (`self.K2_AttachToComponent` (`Character.Mesh` _returnvalue) "PistolaSkt" "SnapToTarget" "SnapToTarget" "SnapToTarget")
  (bind `_aspolicía` (cast `/Game/Policía/Blueprints/Policía` _returnvalue))
  (set `/Game/Policía/Blueprints/Policía.estaArmado` true `_aspolicía`))

(fn `SoltarArma`
  (bind `_aspolicía` (cast `/Game/Policía/Blueprints/Policía` (`GameplayStatics.GetPlayerCharacter` 0)))
  (set `/Game/Policía/Blueprints/Policía.estaArmado` false `_aspolicía`)
  (`self.K2_DetachFromActor` "KeepWorld" "KeepWorld" "KeepWorld"))

(fn `UserConstructionScript`)