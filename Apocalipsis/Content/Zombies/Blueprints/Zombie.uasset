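; Zombie enemy character that chases pawns it sees or hears through PawnSensing and AIMoveTo, and attacks the Policía character.
; Overlapping a Policía starts a looping timer that damages it at the attack rate until overlap ends, while a damage volume toggles the Atacando flag.
; AfectarSalud updates health and plays a hit montage, or on death detaches the controller and destroys the actor after a delay.
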(event `/Game/InterfazDaño.AfectarSalud`
  (params (Delta :type "Float (single-precision)"))
  (bind _capsulecomponent (`self.CapsuleComponent`))
  (bind _salud (`self.Salud`))
  (`self.CalcularSalud` Delta)
  (`KismetSystemLibrary.PrintString` (`KismetStringLibrary.Conv_DoubleToString` _salud))
  (if (> _salud 0.0)
    (`self.PlayAnimMontage` "/Game/Zombies/Animaciones/Zombie_Daño_Montage.Zombie_Daño_Montage" 1.5))
  (if (`self.estaMuerto`)
    (`self.DetachFromControllerPendingDestroy`)
    (`KismetSystemLibrary.Delay` 10.0)
    (`PrimitiveComponent.SetCollisionResponseToChannel` _capsulecomponent "ECC_WorldDynamic" "ECR_Ignore")
    (`PrimitiveComponent.SetCollisionResponseToChannel` _capsulecomponent "ECC_Pawn" "ECR_Ignore")
    (`self.K2_DestroyActor`)))

(event `self.PawnSensing.OnSeePawn`
  (params (Pawn :type "Pawn Object Reference"))
  (`|AIMoveTo` self (0.0 0.0 0.0) Pawn))

(event `self.ReceiveActorBeginOverlap`
  (params (OtherActor :type "Actor Object Reference"))
  (if (`self.estaMuerto`)
    (`KismetSystemLibrary.K2_ClearTimer` null "HacerDañoPolicía" :!label _label)
    (else
      (bind `_aspolicía` (cast `/Game/Policía/Blueprints/Policía` OtherActor))
      (set `self.Policía` `_aspolicía`)
      (`KismetSystemLibrary.K2_SetTimer` null "HacerDañoPolicía" (/ 1.0 (`self.Ataques por segundo`)) true))))

(event `self.PawnSensing.OnHearNoise`
  (params (Instigator :type "Pawn Object Reference") (Location :type "Vector Structure (by ref)") (Volume :type "Float (single-precision)"))
  (`|AIMoveTo` self (0.0 0.0 0.0) Instigator))

(event `self.ReceiveActorEndOverlap`
  (params (OtherActor :type "Actor Object Reference"))
  (if (== OtherActor (`self.Policía`))
    (goto _label)))

(event `HacerDañoPolicía`
  (`/Game/Policía/Blueprints/Policía.AfectarSalud` (`self.Policía`) (`self.Daño`)))

(event `self.Volumen de Daño.OnComponentBeginOverlap`
  (params (OverlappedComponent :type "PrimitiveComponent Object Reference") (OtherActor :type "Actor Object Reference") (OtherComp :type "PrimitiveComponent Object Reference") (OtherBodyIndex :type Integer) (bFromSweep :type Boolean) (SweepResult :type "HitResult Structure (by ref)"))
  (set `self.Atacando` true))

(event `self.Volumen de Daño.OnComponentEndOverlap`
  (params (OverlappedComponent :type "PrimitiveComponent Object Reference") (OtherActor :type "Actor Object Reference") (OtherComp :type "PrimitiveComponent Object Reference") (OtherBodyIndex :type Integer))
  (set `self.Atacando` false))

(fn `UserConstructionScript`)